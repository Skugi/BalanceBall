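; Player pawn that rolls a physics sphere in response to movement input.
; The Left/Right and Forwards/Backwards axes apply torque to Sphere1 around world X and Y respectively, scaled by RollTorque and the axis value.
; Torque is applied as an acceleration change, so the roll response ignores the sphere's mass.
; BeginPlay, overlap, Tick and the construction script contain no logic.
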(event `InputAxis|Left/Right`
  (params (AxisValue :type "Float (single-precision)"))
  (`PrimitiveComponent.AddTorqueInRadians` (`self.Sphere1`) (`KismetMathLibrary.MakeVector` (* (`self.RollTorque`) AxisValue)) "None" true))

(event `InputAxis|Forwards/Backwards`
  (params (AxisValue :type "Float (single-precision)"))
  (`PrimitiveComponent.AddTorqueInRadians` (`self.Sphere1`) (`KismetMathLibrary.MakeVector` 0.0 (* (`self.RollTorque`) AxisValue)) "None" true))

(fn `UserConstructionScript`)