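; BP_WinVolume is a volume actor that checks whether all crystals have been collected when the player overlaps it.
; CheckCrystals passes when GetAllActorsOfClass finds no remaining actors, and the overlap event prints a Polish success or failure message.
; The volume only prints the result, with no further win logic.
; AnyActorsOnLevel repeats the same empty-list check, returning true when none remain despite its name, and is not called here.
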(event `self.ReceiveActorBeginOverlap`
  (params (OtherActor :type "Actor Object Reference"))
  (`/Game/Blueprints/Libraries/ML_Actors.IsPlayer` OtherActor
    (:`True`
      (if (`self.CheckCrystals`)
        (`KismetSystemLibrary.PrintString` "Wszystkie Kryształy zostały zebrane")
        (else
          (`KismetSystemLibrary.PrintString` "Kryształy nie zostały zebrane"))))))

(fn `AnyActorsOnLevel`
  (returns (NewParam :type Boolean))
  (bind _outactors (`GameplayStatics.GetAllActorsOfClass` null))
  (return (>= 0 (`KismetArrayLibrary.Array_Length` _outactors))))

(fn `CheckCrystals`
  (returns (ReturnValue :type Boolean))
  (bind _outactors (`GameplayStatics.GetAllActorsOfClass` null))
  (return (>= 0 (`KismetArrayLibrary.Array_Length` _outactors))))

(fn `UserConstructionScript`)